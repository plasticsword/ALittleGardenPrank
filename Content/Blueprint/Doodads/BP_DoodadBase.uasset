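; Base Blueprint for destructible doodads that swap from an intact sprite to a broken one when health runs out.
; BeginPlay reads max health and an invulnerability flag from a data table row, though UpdateHealth never checks that flag.
; UpdateHealth adds a signed change and spawns a Niagara hit effect.
; On destruction it disables collision, increments the game mode's destroyed count, and ends the game with a win widget if CheckWin passes.
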(event Custom|UpdateHealth
  (params (HealthChange :type Float%20%28double-precision%29))
  (if (not (Variables|Default|GetDestroyed))
    (bind _output_get (Variables|Default|SetHealth (+ HealthChange (Variables|Default|GetHealth))))
    (Niagara|SpawnSystematLocation "/Game/Blueprint/Doodads/NS_DoodadHit.NS_DoodadHit" (Transformation|GetActorLocation))
    (if (<= _output_get 0.0)
      (Variables|Default|SetDestroyed true)
      (Rendering|SetVisibility (Variables|Default|GetSprite) false false)
      (Rendering|SetVisibility (Variables|Default|GetSpriteBroke) true false)
      (Collision|SetCollisionEnabled (Variables|Default|GetCollistion) "NoCollision")
      (bind _asmain_game_mode (Utilities|Casting|CastToMainGameMode (Game|GetGameMode)))
      (Variables|/Game/Blueprint/GameMode/MainGameMode.MainGameMode_C|SetItemsDestroyed _asmain_game_mode (+ (Variables|/Game/Blueprint/GameMode/MainGameMode.MainGameMode_C|GetItemsDestroyed _asmain_game_mode) 1))
      (bind _win (Default|CheckWin _asmain_game_mode))
      (if _win
        (Default|CreateWinWidget _asmain_game_mode)
        (Variables|/Game/Blueprint/GameMode/MainGameMode.MainGameMode_C|SetHasGameEnded _asmain_game_mode true)))))

(event EventBeginPlay
  (bind _datarowhandle (Variables|Default|GetDataRowHandle))
  (bind _returnvalue (Utilities|GetDataTableRow (.datatable _datarowhandle) (.rowname _datarowhandle))
    (:then
      (Variables|Default|SetInvulnerable (.Invulnerable (Utilities|Struct|BreakStruct_Doodads _returnvalue)))
      (bind _output_get (Variables|Default|SetMaxHealth (.MaxHealth (Utilities|Struct|BreakStruct_Doodads _returnvalue))))
      (Variables|Default|SetHealth _output_get)
      (Rendering|SetVisibility (Variables|Default|GetSprite) true false)
      (Rendering|SetVisibility (Variables|Default|GetSpriteBroke) false false))))

(fn ConstructionScript)