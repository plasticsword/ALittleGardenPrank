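; MainGameMode is a game mode Blueprint that provides the HUD, win screen, lose screen and win condition for an item-destruction objective.
; Three functions each create a widget, add it to the viewport and store its reference; the win widget's creation node shows no class.
; CheckWin reports whether ItemsDestroyed has reached MaxItems.
; BeginPlay is empty, and nothing in this Blueprint calls these functions or updates the count.
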(event EventBeginPlay)

(fn ConstructionScript)

(fn CreateLoseWidget
  (bind _returnvalue (UserInterface|CreateWidget "/Game/Blueprint/UI/W_LoseScreen.W_LoseScreen_C"))
  (UserInterface|Viewport|AddtoViewport _returnvalue 0)
  (Variables|Default|SetLoseWidget _returnvalue))

(fn CreateHUD
  (bind _returnvalue (UserInterface|CreateWidget "/Game/Blueprint/UI/W_HUD.W_HUD_C"))
  (UserInterface|Viewport|AddtoViewport _returnvalue 0)
  (Variables|Default|SetHUD _returnvalue))

(fn CheckWin
  (return (>= (Variables|Default|GetItemsDestroyed) (Variables|Default|GetMaxItems))))

(fn CreateWinWidget
  (bind _returnvalue (UserInterface|CreateWidget "/Game/Blueprint/UI/W_WinScreen.W_WinScreen_C"))
  (UserInterface|Viewport|AddtoViewport _returnvalue 0)
  (Variables|Default|SetWinWidget _returnvalue))