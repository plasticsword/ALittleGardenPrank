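; Player-controlled gnome character that walks on world axes, turns toward the mouse cursor and punches doodads with two hands.
; Enhanced Input sets movement, look target and punch flags; Tick interpolates rotation and slides each hand to its target and back.
; Hand overlaps damage BP_DoodadBase actors.
; HandleOnHit applies damage with timed invulnerability; death spawns gibs, hides sprites, ends the game and creates the lose widget.
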(event Custom|OnHandLBeginOverlap
  (params (OverlappedComponent :type Primitive%20Component%20Object%20Reference) (OtherActor :type Actor%20Object%20Reference) (OtherComp :type Primitive%20Component%20Object%20Reference) (OtherBodyIndex :type Integer) (bFromSweep :type Boolean) (SweepResult :type Hit%20Result%20Structure%20%28by%20ref%29))
  (bind _asbp_doodad_base (Utilities|Casting|CastToBP_DoodadBase OtherActor))
  (Default|UpdateHealth _asbp_doodad_base (* (Variables|Default|GetGnomeDamage) -1.0)))

(event Custom|OnHandRBeginOverlap
  (params (OverlappedComponent :type Primitive%20Component%20Object%20Reference) (OtherActor :type Actor%20Object%20Reference) (OtherComp :type Primitive%20Component%20Object%20Reference) (OtherBodyIndex :type Integer) (bFromSweep :type Boolean) (SweepResult :type Hit%20Result%20Structure%20%28by%20ref%29))
  (bind _asbp_doodad_base (Utilities|Casting|CastToBP_DoodadBase OtherActor))
  (Default|UpdateHealth _asbp_doodad_base (* (Variables|Default|GetGnomeDamage) -1.0)))

(event Input|EnhancedActionEvents|EnhancedInputActionIA_Move
  (params (ActionValue :type Vector%202D%20Structure) (ElapsedSeconds :type Float%20%28double-precision%29) (TriggeredSeconds :type Float%20%28double-precision%29) (InputAction :type Input%20Action%20Object%20Reference :default "/Game/Blueprint/Input/Actions/IA_Move.IA_Move"))
  ;[1 1 1] Comment
  (bind _asmain_game_mode (Utilities|Casting|CastToMainGameMode (Game|GetGameMode)))
  (if (not (Variables|/Game/Blueprint/GameMode/MainGameMode.MainGameMode_C|GetHasGameEnded _asmain_game_mode))
    (Pawn|Input|AddMovementInput (Math|Vector|GetForwardVector "0, 0, 0") (.x ActionValue) false)
    (Pawn|Input|AddMovementInput (Math|Vector|GetRightVector "0, 0, 0") (.y ActionValue) false)))

(event Input|EnhancedActionEvents|EnhancedInputActionIA_Look
  (params (ActionValue :type Vector%202D%20Structure) (ElapsedSeconds :type Float%20%28double-precision%29) (TriggeredSeconds :type Float%20%28double-precision%29) (InputAction :type Input%20Action%20Object%20Reference :default "/Game/Blueprint/Input/Actions/IA_Look.IA_Look"))
  (bind _returnvalue (Transformation|GetActorLocation))
  (bind _gnomecontroller (Variables|Default|GetGnomeController))
  (bind _hitresult (Game|Player|GetHitResultUnderCursorbyChannel _gnomecontroller "TraceTypeQuery1" true))
  ;[1 1 1] Comment
  (Variables|Default|SetLookAtRotation (Math|Rotator|FindLookatRotation (Math|Vector|MakeVector (.x _returnvalue) (.y _returnvalue) 0.0) (Math|Vector|MakeVector (.x (.location _hitresult)) (.y (.location _hitresult)) 0.0))))

(event Input|EnhancedActionEvents|EnhancedInputActionIA_HandL
  (params (ActionValue :type Boolean) (ElapsedSeconds :type Float%20%28double-precision%29) (TriggeredSeconds :type Float%20%28double-precision%29) (InputAction :type Input%20Action%20Object%20Reference :default "/Game/Blueprint/Input/Actions/IA_HandL.IA_HandL"))
  (Variables|Default|SetHandLMoving true))

(event Input|EnhancedActionEvents|EnhancedInputActionIA_HandR
  (params (ActionValue :type Boolean) (ElapsedSeconds :type Float%20%28double-precision%29) (TriggeredSeconds :type Float%20%28double-precision%29) (InputAction :type Input%20Action%20Object%20Reference :default "/Game/Blueprint/Input/Actions/IA_HandR.IA_HandR"))
  (Variables|Default|SetHandRMoving true))

(event EventBeginPlay
  (bind _asmain_game_mode (Utilities|Casting|CastToMainGameMode (Game|GetGameMode)))
  (bind _asw_hud (Utilities|Casting|CastToW_HUD (Variables|/Game/Blueprint/GameMode/MainGameMode.MainGameMode_C|GetHUD _asmain_game_mode)))
  (Default|SetGnome _asw_hud self)
  (bind _output_get (Variables|Default|SetGnomeController (Game|GetPlayerController 0)))
  (bind _asbp_gnome_controller (Utilities|Casting|CastToBP_GnomeController _output_get))
  (Input|AddMappingContext (PlayerController|LocalPlayerSubsystems|GetEnhancedInputLocalPlayerSubsystem _asbp_gnome_controller) "/Game/Blueprint/Input/IMC_Gnome.IMC_Gnome" 0 "(bIgnoreAllPressedKeysUntilRelease=True,bForceImmediately=False,bNotifyUserSettings=False)")
  (Variables|/Script/Engine.PlayerController|SetbShowMouseCursor (Variables|Default|GetGnomeController) true)
  (Variables|Default|SetHandRDefaultLocation (Variables|/Script/Engine.SceneComponent|GetRelativeLocation (Variables|Default|GetHandR)))
  (Variables|Default|SetHandLDefaultLocation (Variables|/Script/Engine.SceneComponent|GetRelativeLocation (Variables|Default|GetHandL)))
  (Utilities|FlowControl|Sequence
    (:then_0
      (Collision|AssignOnComponentBeginOverlap (Variables|Default|GetHandR) (delegate Custom|OnHandRBeginOverlap)))
    (:then_1
      (Collision|AssignOnComponentBeginOverlap (Variables|Default|GetHandL) (delegate Custom|OnHandLBeginOverlap)))))

(event EventTick
  (params (DeltaSeconds :type Float%20%28single-precision%29))
  (bind _handr (Variables|Default|GetHandR))
  (bind _handr_2 (Variables|Default|GetHandR))
  (bind _handl (Variables|Default|GetHandL))
  (bind _handl_2 (Variables|Default|GetHandL))
  (bind _asmain_game_mode (Utilities|Casting|CastToMainGameMode (Game|GetGameMode)))
  (if (not (Variables|/Game/Blueprint/GameMode/MainGameMode.MainGameMode_C|GetHasGameEnded _asmain_game_mode))
    ;[1 1 1] Comment
    (Input|SetInputModeGameOnly (Variables|Default|GetGnomeController) false)
    (Transformation|SetActorRotation (Class|KismetMathLibrary|RInterptoConstant (Transformation|GetActorRotation) (Variables|Default|GetLookAtRotation) DeltaSeconds (Variables|Default|GetGnomeTurnSpeed)))
    (Utilities|FlowControl|Sequence
      (:then_0
        ;[1 1 1] Comment
        (if (Variables|Default|GetHandLMoving)
          (Transformation|SetRelativeLocation _handl (Math|Interpolation|VInterptoConstant (Variables|/Script/Engine.SceneComponent|GetRelativeLocation _handl) (Variables|/Script/Engine.SceneComponent|GetRelativeLocation (Variables|Default|GetHandLTarget)) DeltaSeconds 3e+02) false false)
          (if (Utilities|Operators|EqualEqual (Variables|/Script/Engine.SceneComponent|GetRelativeLocation (Variables|Default|GetHandL)) (Variables|/Script/Engine.SceneComponent|GetRelativeLocation (Variables|Default|GetHandLTarget)) 1.0)
            (Variables|Default|SetHandLMoving false))
          (elif (not (Utilities|Operators|EqualEqual (Variables|/Script/Engine.SceneComponent|GetRelativeLocation (Variables|Default|GetHandL)) (Variables|Default|GetHandLDefaultLocation) 1.0))
            (Transformation|SetRelativeLocation _handl_2 (Math|Interpolation|VInterptoConstant (Variables|/Script/Engine.SceneComponent|GetRelativeLocation _handl_2) (Variables|Default|GetHandLDefaultLocation) DeltaSeconds 3e+02) false false))))
      (:then_1
        ;[1 1 1] Comment
        (if (Variables|Default|GetHandRMoving)
          (Transformation|SetRelativeLocation _handr_2 (Math|Interpolation|VInterptoConstant (Variables|/Script/Engine.SceneComponent|GetRelativeLocation _handr_2) (Variables|/Script/Engine.SceneComponent|GetRelativeLocation (Variables|Default|GetHandRTarget)) DeltaSeconds 3e+02) false false)
          (if (Utilities|Operators|EqualEqual (Variables|/Script/Engine.SceneComponent|GetRelativeLocation (Variables|Default|GetHandR)) (Variables|/Script/Engine.SceneComponent|GetRelativeLocation (Variables|Default|GetHandRTarget)) 1.0)
            (Variables|Default|SetHandRMoving false))
          (elif (not (Utilities|Operators|EqualEqual (Variables|/Script/Engine.SceneComponent|GetRelativeLocation (Variables|Default|GetHandR)) (Variables|Default|GetHandRDefaultLocation) 1.0))
            (Transformation|SetRelativeLocation _handr (Math|Interpolation|VInterptoConstant (Variables|/Script/Engine.SceneComponent|GetRelativeLocation _handr) (Variables|Default|GetHandRDefaultLocation) DeltaSeconds 3e+02) false false)))))))

(fn ConstructionScript)

(fn HandleonHit
  (params (damage :type Float%20%28double-precision%29))
  (if (not (Variables|Default|GetIsIFrame))
    (Variables|Default|SetIsIFrame true)
    (bind _output_get (Variables|Default|SetHealth (- (Variables|Default|GetHealth) damage)))
    (Utilities|Time|SetTimerbyEvent (EventDispatchers|CreateEvent :!event ResetIFrame) 0.5)
    (if (<= _output_get 0.0)
      (Variables|Default|SetIsDead true)
      (Niagara|SpawnSystematLocation "/Game/Blueprint/Character/Gnome/NS_GnomeGibs.NS_GnomeGibs" (Transformation|GetActorLocation))
      (bind _asmain_game_mode (Utilities|Casting|CastToMainGameMode (Game|GetGameMode)))
      (Variables|/Game/Blueprint/GameMode/MainGameMode.MainGameMode_C|SetHasGameEnded _asmain_game_mode true)
      (for _array_element (Actor|GetComponentsByClass "/Script/Paper2D.PaperSpriteComponent")
        (Rendering|SetVisibility _array_element false false)
        (Default|CreateLoseWidget _asmain_game_mode)))))

(fn ResetIFrame
  (Variables|Default|SetIsIFrame false))