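; Jon is an enemy that chases the player pawn, attacks with two hands and periodically rests.
; It overrides parent chase, range and attack functions, interpolating both hands toward HandLTarget and back, with right-hand overlaps damaging BP_Gnome.
; A looping timer toggles resting, which pauses movement and attacks and shows Sleep; changing RestTimer never re-arms it.
; The timer is cleared if a hit finds the game ended.
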(event Custom|Resting
  (bind _sleep (Variables|Default|GetSleep))
  (bind _output_get (Variables|Default|SetIsResting (not (Variables|Default|GetIsResting))))
  (if _output_get
    (Variables|Default|SetRestTimer 5.0)
    (Rendering|SetVisibility _sleep true false)
    (else
      (Variables|Default|SetRestTimer 8.0)
      (Rendering|SetVisibility _sleep false false))))

(event Custom|OnHit
  (params (OverlappedComponent :type Primitive%20Component%20Object%20Reference) (OtherActor :type Actor%20Object%20Reference) (OtherComp :type Primitive%20Component%20Object%20Reference) (OtherBodyIndex :type Integer) (bFromSweep :type Boolean) (SweepResult :type Hit%20Result%20Structure%20%28by%20ref%29))
  (bind _asbp_gnome (Utilities|Casting|CastToBP_Gnome OtherActor))
  (Default|HandleonHit _asbp_gnome (Variables|Default|GetDamage))
  (bind _asmain_game_mode (Utilities|Casting|CastToMainGameMode (Game|GetGameMode)))
  (if (Variables|/Game/Blueprint/GameMode/MainGameMode.MainGameMode_C|GetHasGameEnded _asmain_game_mode)
    (Utilities|Time|ClearandInvalidateTimerbyHandle (Variables|Default|GetRestTimerHandle))))

(event EventBeginPlay
  (Utilities|FlowControl|Sequence
    (:then_0
      (Variables|Default|SetState "NewEnumerator2")
      (Variables|Default|SetHandRDefaultLocation (Variables|/Script/Engine.SceneComponent|GetRelativeLocation (Variables|Default|GetHandR)))
      (Variables|Default|SetHandLDefaultLocation (Variables|/Script/Engine.SceneComponent|GetRelativeLocation (Variables|Default|GetHandL)))
      (bind _returnvalue (Utilities|Time|SetTimerbyEvent (delegate Custom|Resting) (Variables|Default|GetRestTimer) true))
      (Variables|Default|SetRestTimerHandle _returnvalue))
    (:then_1
      (Collision|BindEventtoOnComponentBeginOverlap (Variables|Default|GetHandR) (delegate Custom|OnHit)))))

(fn ConstructionScript
  (|CallParentFunction))

(fn Chase
  (params (delta :type Float%20%28double-precision%29))
  (bind _returnvalue (Game|Player|GetPlayerPawn 0))
  (bind _returnvalue_2 (Transformation|GetActorLocation))
  (bind _returnvalue_3 (Transformation|GetActorLocation _returnvalue))
  (if (not (Variables|Default|GetIsResting))
    (Transformation|SetActorRotation (Math|Rotator|FindLookatRotation (Transformation|GetActorLocation) (Transformation|GetActorLocation _returnvalue)))
    (if (not (<= (Math|Vector|VectorLength (- (Transformation|GetActorLocation) (Transformation|GetActorLocation _returnvalue))) 85.0))
      (Transformation|SetActorLocation (Math|Interpolation|VInterptoConstant (Math|Vector|MakeVector (.x _returnvalue_2) (.y _returnvalue_2) (.z _returnvalue_2)) (Math|Vector|MakeVector (.x _returnvalue_3) (.y _returnvalue_3) (.z _returnvalue_2)) delta 5.5e+02) false false)
      (|CallParentFunction delta))))

(fn IsWithinRange
  (|CallParentFunction)
  (return (<= (Math|Vector|VectorLength (- (Transformation|GetActorLocation (Game|Player|GetPlayerPawn 0)) (Transformation|GetWorldLocation (Variables|Default|GetHandRTarget)))) 5e+01)))

(fn BeginAttack
  (params (delta :type Float%20%28double-precision%29))
  (if (not (Variables|Default|GetIsAttacking))
    (Variables|Default|SetIsAttacking true)
    (Variables|Default|SetHandMoving true)))

(fn UpdateAttack
  (params (delta :type Float%20%28double-precision%29))
  (bind _handl (Variables|Default|GetHandL))
  (bind _handr (Variables|Default|GetHandR))
  (bind _handr_2 (Variables|Default|GetHandR))
  (bind _handl_2 (Variables|Default|GetHandL))
  (if (and (Variables|Default|GetIsAttacking) (not (Variables|Default|GetIsResting)))
    ;[1 1 1] Comment
    (if (Variables|Default|GetHandMoving)
      (Utilities|FlowControl|Sequence
        (:then_0
          (Transformation|SetRelativeLocation _handl (Math|Interpolation|VInterptoConstant (Variables|/Script/Engine.SceneComponent|GetRelativeLocation _handl) (Variables|/Script/Engine.SceneComponent|GetRelativeLocation (Variables|Default|GetHandLTarget)) delta 3e+02) false false))
        (:then_1
          (Transformation|SetRelativeLocation _handr (Math|Interpolation|VInterptoConstant (Variables|/Script/Engine.SceneComponent|GetRelativeLocation _handr) (Variables|/Script/Engine.SceneComponent|GetRelativeLocation (Variables|Default|GetHandLTarget)) delta 3e+02) false false))
        (:then_2
          (if (Utilities|Operators|EqualEqual (Variables|/Script/Engine.SceneComponent|GetRelativeLocation (Variables|Default|GetHandL)) (Variables|/Script/Engine.SceneComponent|GetRelativeLocation (Variables|Default|GetHandLTarget)) 1.0)
            (Variables|Default|SetHandMoving false))))
      (elif (Utilities|Operators|EqualEqual (Variables|/Script/Engine.SceneComponent|GetRelativeLocation (Variables|Default|GetHandL)) (Variables|Default|GetHandLDefaultLocation) 1.0)
        (Variables|Default|SetIsAttacking false)
        (else
          (Utilities|FlowControl|Sequence
            (:then_0
              (Transformation|SetRelativeLocation _handl_2 (Math|Interpolation|VInterptoConstant (Variables|/Script/Engine.SceneComponent|GetRelativeLocation _handl_2) (Variables|Default|GetHandLDefaultLocation) delta 3e+02) false false))
            (:then_1
              (Transformation|SetRelativeLocation _handr_2 (Math|Interpolation|VInterptoConstant (Variables|/Script/Engine.SceneComponent|GetRelativeLocation _handr_2) (Variables|Default|GetHandRDefaultLocation) delta 3e+02) false false))))))))