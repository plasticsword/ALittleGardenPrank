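; BP_EnemyBase is a base enemy Blueprint that provides the per-tick chase and attack skeleton for child enemies.
; While MainGameMode reports the game has not ended, the Chase state runs Chase, then calls BeginAttack if IsWithinRange passes.
; UpdateAttack runs every such tick regardless of state.
; Chase, BeginAttack and UpdateAttack are empty stubs and IsWithinRange returns false, leaving behavior to overrides.
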(event EventTick
  (params (DeltaSeconds :type Float%20%28single-precision%29))
  (bind _asmain_game_mode (Utilities|Casting|CastToMainGameMode (Game|GetGameMode)))
  (if (not (Variables|/Game/Blueprint/GameMode/MainGameMode.MainGameMode_C|GetHasGameEnded _asmain_game_mode))
    (Utilities|FlowControl|Sequence
      (:then_0
        (switch Utilities|FlowControl|Switch|SwitchonE_EnemyState (Variables|Default|GetState)
          (:NewEnumerator2
            (CallFunction|Chase DeltaSeconds)
            (bind _newparam (CallFunction|IsWithinRange))
            (if _newparam
              (CallFunction|BeginAttack DeltaSeconds)))))
      (:then_1
        (CallFunction|UpdateAttack DeltaSeconds)))))

(fn ConstructionScript)

(fn Chase
  (params (delta :type Float%20%28double-precision%29)))

(fn BeginAttack
  (params (delta :type Float%20%28double-precision%29)))

(fn IsWithinRange
  (return false))

(fn UpdateAttack
  (params (delta :type Float%20%28double-precision%29)))